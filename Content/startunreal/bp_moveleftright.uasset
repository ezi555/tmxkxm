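; Blueprint actor that slides its Sphere component along relative axes, scaled by a Speed variable and frame time.
; Tick moves it along X while Isrightmove is set, otherwise along Z if Isupmove is set.
; Tick's limit checks never reverse motion: the X branch immediately re-sets Isrightmove to true, and the Z check is empty.
; A second graph's CustomEvent, uncalled here, toggles between X and Y movement at set limits.
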(event `self.ReceiveTick`
  (params (DeltaSeconds :type "Float (single-precision)"))
  (bind _sphere (`self.Sphere`))
  (bind _returnvalue (* DeltaSeconds (`self.speed`)))
  (bind (_relativelocation_x _relativelocation_y _relativelocation_z) (`KismetMathLibrary.BreakVector` (`SceneComponent.RelativeLocation` _sphere)))
  (bind _relativelocation_x_2 (`KismetMathLibrary.BreakVector` (`SceneComponent.RelativeLocation` _sphere)))
  (if (`self.isrightmove`)
    (`SceneComponent.K2_AddRelativeLocation` _sphere (`KismetMathLibrary.MakeVector` _returnvalue) false false)
    (if (> _relativelocation_x_2 100.0)
      (set `self.isrightmove` false)
      (set `self.isrightmove` true))
    (elif (`self.isupmove`)
      (`SceneComponent.K2_AddRelativeLocation` _sphere (`KismetMathLibrary.MakeVector` 0.0 0.0 _returnvalue) false false)
      (if (> _relativelocation_z 100.0)
        _))))

(event `CustomEvent`
  (params (DeltaSeconds :type "Float (double-precision)"))
  (bind _sphere (`self.Sphere`))
  (bind _returnvalue (* DeltaSeconds (`self.speed`)))
  (bind (_relativelocation_x _relativelocation_y) (`KismetMathLibrary.BreakVector` (`SceneComponent.RelativeLocation` _sphere)))
  (bind _relativelocation_x_2 (`KismetMathLibrary.BreakVector` (`SceneComponent.RelativeLocation` _sphere)))
  (if (`self.isrightmove`)
    (`SceneComponent.K2_AddRelativeLocation` _sphere (`KismetMathLibrary.MakeVector` _returnvalue) false false)
    (if (> _relativelocation_x_2 100.0)
      (set `self.isrightmove` false))
    (else
      (bind _result (`/Engine/EditorBlueprintResources/StandardMacros.NegateFloat` _returnvalue)
        (:`  `
          (`SceneComponent.K2_AddRelativeLocation` _sphere (`KismetMathLibrary.MakeVector` 0.0 _result) false false)
          (if (<= _relativelocation_y 0.0)
            (set `self.isrightmove` true)))))))

(fn `UserConstructionScript`)