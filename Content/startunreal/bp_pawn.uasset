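; Practice Pawn Blueprint with basic axis-driven movement, look controls and debug printing of key presses and elapsed time.
; Tick accumulates delta time, printing each new whole second in Korean and resetting at 59; an uncalled Showtimesec function duplicates this with reversed branches.
; Movement offsets the actor along forward and right vectors without sweep or delta-time scaling.
; LookUp feeds controller yaw and Lookright feeds pitch, opposite to their names.
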(event `self.ReceiveBeginPlay`
  (`KismetSystemLibrary.PrintString` "BeginPlay" true true (struct :`G` 0.66 :`B` 1.0 :`A` 1.0) 1.0))

(event `self.ReceiveTick`
  (params (DeltaSeconds :type "Float (single-precision)"))
  (bind _output_get (set `self.TotalDeltaSeconds` (+ DeltaSeconds (`self.TotalDeltaSeconds`))))
  (bind _returnvalue (`KismetMathLibrary.FFloor` _output_get))
  (if (== (`self.beforeint`) _returnvalue)
    _
    (elif (< _returnvalue 59)
      (`KismetSystemLibrary.PrintString` (`KismetStringLibrary.Concat_StrStr` (`KismetStringLibrary.Conv_IntToString` _returnvalue) "초") true true (struct :`G` 0.66 :`B` 1.0 :`A` 1.0) 1.0)
      (set `self.beforeint` _returnvalue)
      (else
        (set `self.TotalDeltaSeconds` 0.0)))))

(event `Key|W`
  (params (Key :type "Key Structure"))
  (:`Pressed`
    (`KismetSystemLibrary.PrintString` "W 키 Pressed")))

(event `InputAction|Enterinput`
  (params (Key :type "Key Structure"))
  (:`Pressed`
    (`KismetSystemLibrary.PrintString` "Enter 키 Pressed")))

(event `InputAxis|moveForward`
  (params (AxisValue :type "Float (single-precision)"))
  ;[1 1 1] 앞쪽으로의 움직임
  (`self.K2_AddActorWorldOffset` (* (`self.GetActorForwardVector`) (* AxisValue 10.0))))

(event `InputAxis|moveright`
  (params (AxisValue :type "Float (single-precision)"))
  ;[1 1 1] 옆쪽으로의 움직임
  (`self.K2_AddActorWorldOffset` (* (`self.GetActorRightVector`) (* AxisValue 10.0))))

(event `InputAxis|LookUp`
  (params (AxisValue :type "Float (single-precision)"))
  (`self.AddControllerYawInput` AxisValue))

(event `InputAxis|Lookright`
  (params (AxisValue :type "Float (single-precision)"))
  (`self.AddControllerPitchInput` AxisValue))

(fn `showtimesec`
  (params (`Delta Seconds` :type "Float (double-precision)"))
  (bind _output_get (set `self.TotalDeltaSeconds` (+ `Delta Seconds` (`self.TotalDeltaSeconds`))))
  (bind _returnvalue (`KismetMathLibrary.FFloor` _output_get))
  (if (== (`self.beforeint`) _returnvalue)
    _
    (elif (< _returnvalue 59)
      (set `self.TotalDeltaSeconds` 0.0)
      (else
        (`KismetSystemLibrary.PrintString` (`KismetStringLibrary.Concat_StrStr` (`KismetStringLibrary.Conv_IntToString` _returnvalue) "초"))
        (set `self.beforeint` _returnvalue)))))

(fn `UserConstructionScript`)